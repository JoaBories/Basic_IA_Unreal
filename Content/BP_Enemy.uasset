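; Enemy Blueprint with health, a montage attack and an overhead-style health bar widget that rotates each tick toward the player.
; TakeDamage and Heal clamp HP and refresh the bar through UpdateLife.
; Damage also drives AI by writing the blackboard State enum: one state at half health or below, otherwise another on a coin flip.
; Attack signals montage completion through OnAttackAnimEnded; ChangeState retains a debug print.
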(event `self.ReceiveTick`
  (params (DeltaSeconds :type "Float (single-precision)"))
  (`SceneComponent.K2_SetWorldRotation` (`self.HealthBar`) (`KismetMathLibrary.FindLookAtRotation` (`SceneComponent.K2_GetComponentLocation` (`self.HealthBar`)) (`self.K2_GetActorLocation` (cast `/Game/ThirdPerson/Blueprints/BP_ThirdPersonCharacter` (`GameplayStatics.GetPlayerCharacter` 0) :!pure true))) false false))

(event `Attack`
  (`|PlayMontage` (`self.Mesh`) "/Game/Characters/Mannequins/Anims/Unarmed/Attack/AM_Attack1.AM_Attack1"
    (:`OnCompleted`
      (`self.OnAttackAnimEnded`))))

(event `self.ReceiveBeginPlay`
  (set `self.CurrentHP` (`self.MaxHp`))
  (`self.UpdateLife`))

(event `/Game/BPI_Damage.TakeDamage`
  (params (Damage :type "Float (double-precision)"))
  (bind _output_get (set `self.CurrentHP` (- (`self.CurrentHP`) Damage)))
  (if (< _output_get 0.0)
    (set `self.CurrentHP` 0.0))
  (`self.UpdateLife`)
  (if (<= (`self.CurrentHP`) (/ (`self.MaxHp`) 2.0))
    (`self.ChangeState` "NewEnumerator5")
    (elif (`KismetMathLibrary.RandomBool`)
      (`self.ChangeState` "NewEnumerator4"))))

(event `/Game/BPI_Damage.Heal`
  (params (Amount :type "Float (double-precision)"))
  (bind _output_get (set `self.CurrentHP` (+ (`self.CurrentHP`) Amount)))
  (if (> _output_get (`self.MaxHp`))
    (set `self.CurrentHP` (`self.MaxHp`)))
  (`self.UpdateLife`))

(fn `ChangeState`
  (params (NewState :type "/Game/E_EnemyState Enum" :default "NewEnumerator0"))
  (`BlackboardComponent.SetValueAsEnum` (`AIBlueprintHelperLibrary.GetBlackboard` null) "State" NewState)
  (`KismetSystemLibrary.PrintString` "Hello"))

(fn `UpdateLife`
  (bind _aswbp_health_bar (cast `/Game/WBP_HealthBar` (`WidgetComponent.GetWidget` (`self.HealthBar`))))
  (`ProgressBar.SetPercent` (`/Game/WBP_HealthBar.ProgressBar_27` _aswbp_health_bar) (/ (`self.CurrentHP`) (`self.MaxHp`))))

(fn `UserConstructionScript`)